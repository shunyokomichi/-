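; Game mode that runs a timed session across three streamed stages, opening the Result level when the time limit expires.
; BeginPlay loads Stage1, moves the player to a PlayerStart, adds two widgets (hiding the fade shortly after) and increments NSpeed every second.
; NEXT and NextStage swap in later stages and reposition the player.
; Respawn binds to pawn destruction, possesses a fresh BP_Player, then rebinds itself.
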(event `self.ReceiveTick`
  (params (DeltaSeconds :type "Float (single-precision)"))
  (bind _output_get (set `self.fTime` (+ DeltaSeconds (`self.fTime`))))
  (if (>= _output_get 60.0)
    (`GameplayStatics.OpenLevel` "Result")))

(event `リスポーンイベント`
  (add `self.OnDestroyed` (`GameplayStatics.GetPlayerPawn` 0) (delegate `リスポーンプレイヤー`)))

(event `リスポーンプレイヤー` :!signature `self.OnDestroyed`
  (params (DestroyedActor :type "Actor Object Reference"))
  (bind _returnvalue (`GameplayStatics.GetPlayerController` 0))
  (bind _returnvalue_2 (`|SpawnActorFromClass` "/Game/BluePrint/player/BP_Player.BP_Player_C" (`self.GetTransform` (`self.K2_FindPlayerStart` null)) "Undefined" "OverrideRootScale" null null)) ; プレイヤーの生成
  (`Controller.Possess` _returnvalue _returnvalue_2)
  (`PlayerController.SetAudioListenerOverride` :`self` _returnvalue)
  (`self.リスポーンイベント`))

(event `self.ReceiveBeginPlay`
  (`GameplayStatics.LoadStreamLevel` "Stage1" true true)
  (`self.リスポーンイベント`) ; リスポーンイベントの呼び出し
  (`self.K2_SetActorTransform` (`GameplayStatics.GetPlayerPawn` 0) (`self.GetTransform` (`self.K2_FindPlayerStart` null)) false false)
  (bind _returnvalue (`|CreateWidget` "/Game/BluePrint/BP_Lade.BP_Lade_C"))
  (`UserWidget.AddToViewport` _returnvalue 0)
  (`KismetSystemLibrary.K2_SetTimerDelegate` (delegate `Add`) 1.0 true)
  (bind _returnvalue_2 (`|CreateWidget` "/Game/BluePrint/BP_Fade.BP_Fade_C"))
  (`UserWidget.AddToViewport` _returnvalue_2 0)
  (bind _output_get (set `self.NewVar_0` _returnvalue_2))
  (`KismetSystemLibrary.Delay` 1.0)
  (`Widget.SetVisibility` _output_get "Hidden"))

(event `Add`
  (set `self.NSpeed` (+ (`self.NSpeed`) 1)))

(event `NEXT`
  (`GameplayStatics.UnloadStreamLevel` "Stage1")
  (`GameplayStatics.LoadStreamLevel` "Stage2" true true)
  (`self.K2_SetActorTransform` (`GameplayStatics.GetPlayerPawn` 0) (`self.GetTransform` (`self.K2_FindPlayerStart` null)) false false))

(event `NextStage`
  (`GameplayStatics.UnloadStreamLevel` "Stage2")
  (`GameplayStatics.LoadStreamLevel` "Stage3" true true)
  (`self.K2_SetActorTransform` (`GameplayStatics.GetPlayerPawn` 0) (`self.GetTransform` (`self.K2_FindPlayerStart` null)) false false))

(fn `UserConstructionScript`)