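; BP_Skeleton is a skeleton hazard that punishes the player on contact and turns 180 degrees whenever its capsule hits something.
; A capsule overlap with BP_Player slows the player, calls DamagePlayer, then triggers the player's fade-out and color change.
; A FlipFlop on that overlap alternately spawns a BP_Hit actor at the player's transform and destroys it on the next overlap.
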(event `self.ReceiveTick`
  (params (DeltaSeconds :type "Float (single-precision)")))

(event `self.CapsuleComponent.OnComponentHit`
  (params (HitComponent :type "PrimitiveComponent Object Reference") (OtherActor :type "Actor Object Reference") (OtherComp :type "PrimitiveComponent Object Reference") (NormalImpulse :type "Vector Structure") (Hit :type "HitResult Structure (by ref)"))
  (`self.K2_SetActorRelativeRotation` (`KismetMathLibrary.ComposeRotators` (`self.K2_GetActorRotation`) (struct :`Yaw` 180.0))))

(event `self.CapsuleComponent.OnComponentBeginOverlap`
  (params (OverlappedComponent :type "PrimitiveComponent Object Reference") (OtherActor :type "Actor Object Reference") (OtherComp :type "PrimitiveComponent Object Reference") (OtherBodyIndex :type Integer) (bFromSweep :type Boolean) (SweepResult :type "HitResult Structure (by ref)"))
  (bind _asbp_player (cast `/Game/BluePrint/player/BP_Player` OtherActor))
  (`/Game/BluePrint/player/BP_Player.Speed_Down` _asbp_player)
  (`/Game/BluePrint/BP_Damage.Damage Player` null)
  (`/Game/BluePrint/player/BP_Player.Fade Out` _asbp_player)
  (`/Game/BluePrint/player/BP_Player.ApplyColor` _asbp_player)
  (`/Engine/EditorBlueprintResources/StandardMacros.FlipFlop`
    (:`A`
      (bind _returnvalue (`|SpawnActorFromClass` "/Game/BluePrint/player/BP_Hit.BP_Hit_C" (`self.GetTransform` (`GameplayStatics.GetPlayerCharacter` 0)) "Undefined" "OverrideRootScale" null null))
      (set `self.Hit` _returnvalue))
    (:`B`
      (`self.K2_DestroyActor` (`self.Hit`)))))

(fn `UserConstructionScript`)