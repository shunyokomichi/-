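; BP_Trapwall is a trap that periodically launches physics-driven rocks from a pit toward a receiving hole.
; The construction script aims Pit at HoleEnd and adds a mesh there facing back, stored as Hold.
; A looping timer spawns BP_Rock relative to the Arrow and applies a velocity-change impulse along its forward axis.
; Rocks overlapping Hold get a very short lifespan, so they vanish almost immediately.
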(event `self.ReceiveBeginPlay`
  (`KismetSystemLibrary.K2_SetTimerDelegate` (delegate `すぽ`) 3.0 true))

(event `すぽ`
  (bind _returnvalue (`SceneComponent.K2_GetComponentToWorld` (`self.Arrow`)))
  (bind _returnvalue_2 (`|SpawnActorFromClass` "/Game/BluePrint/MODEL/BP_Rock.BP_Rock_C" (`KismetMathLibrary.MakeTransform` (`KismetMathLibrary.TransformLocation` _returnvalue (100.0 0.0 -100.0)) (.rotation _returnvalue) (.scale _returnvalue)) "Undefined" "OverrideRootScale" null null))
  (bind _rock (`/Game/BluePrint/MODEL/BP_Rock.rock` _returnvalue_2))
  (`PrimitiveComponent.SetSimulatePhysics` _rock true)
  (`PrimitiveComponent.AddImpulse` _rock (`KismetMathLibrary.TransformDirection` _returnvalue (2500.0 0.0 0.0)) "None" true))

(event `self.Hold.OnComponentBeginOverlap`
  (params (OverlappedComponent :type "PrimitiveComponent Object Reference") (OtherActor :type "Actor Object Reference") (OtherComp :type "PrimitiveComponent Object Reference") (OtherBodyIndex :type Integer) (bFromSweep :type Boolean) (SweepResult :type "HitResult Structure (by ref)"))
  (bind _asbp_rock (cast `/Game/BluePrint/MODEL/BP_Rock` OtherActor))
  (`self.SetLifeSpan` _asbp_rock 0.09))

(fn `UserConstructionScript`
  (bind _holeend (`self.holeEnd`))
  (bind _pit (`self.pit`))
  (bind _relativelocation (`SceneComponent.RelativeLocation` _pit))
  (`SceneComponent.K2_SetRelativeRotation` _pit (`KismetMathLibrary.FindLookAtRotation` _relativelocation _holeend) false false)
  (bind _returnvalue (`AddComponent|NODE_AddStaticMeshComponent-0` :`RelativeTransform` (`KismetMathLibrary.MakeTransform` _holeend (`KismetMathLibrary.FindLookAtRotation` _holeend _relativelocation))))
  (set `self.Hold` _returnvalue))