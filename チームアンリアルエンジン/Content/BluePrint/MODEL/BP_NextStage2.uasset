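; BP_NextStage2 is a trigger volume that advances the player to the next stage when they reach it.
; When a BP_Player overlaps its Box, it prints a debug string and calls NextStage on BP_GAMEMODE.
; If its LastStage flag is set, it also marks Clear on the custom game instance and opens the RESULT level.
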(event `self.Box.OnComponentBeginOverlap`
  (params (OverlappedComponent :type "PrimitiveComponent Object Reference") (OtherActor :type "Actor Object Reference") (OtherComp :type "PrimitiveComponent Object Reference") (OtherBodyIndex :type Integer) (bFromSweep :type Boolean) (SweepResult :type "HitResult Structure (by ref)"))
  (cast `/Game/BluePrint/player/BP_Player` OtherActor)
  (`KismetSystemLibrary.PrintString` "Hello")
  (`/Game/BluePrint/BP_GAMEMODE.NextStage` (cast `/Game/BluePrint/BP_GAMEMODE` (`GameplayStatics.GetGameMode`) :!pure true))
  (if (`self.bLastStage`)
    (set `/Game/BluePrint/BP_Castom_Game_Instans.bClear` true (cast `/Game/BluePrint/BP_Castom_Game_Instans` (`GameplayStatics.GetGameInstance`) :!pure true))
    (`GameplayStatics.OpenLevel` "RESULT")))

(fn `UserConstructionScript`)